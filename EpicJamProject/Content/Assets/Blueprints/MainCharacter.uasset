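; MainCharacter is an actor that rides along a track like a cart when its ActiveCart flag is set at BeginPlay.
; MoveCart scales the CartMover timeline's play rate by Duration and starts it at StartOffset.
; Each timeline update maps Alpha to a distance along the TrackRef spline and sets the actor's world location and rotation to match.
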(event Custom|MoveCart
  (bind _trackref (Variables|Default|GetTrackRef))
  (bind _cartmover (Variables|Default|GetCartMover))
  (bind _path (Variables|/Game/Assets/Blueprints/Track.Track_C|GetPath _trackref))
  (Components|Timeline|SetPlayRate _cartmover (/ 1.0 (Variables|Default|GetDuration)))
  (Components|Timeline|SetNewTime _cartmover (Variables|Default|GetStartOffset))
  (bind _alpha (Timeline|CartMover Play)
    (:Update
      (Variables|Default|SetAlpha _alpha)
      (Transformation|SetActorLocationAndRotation (Spline|GetLocationatDistanceAlongSpline _path (Math|Float|Lerp 0.0 (Spline|GetSplineLength _path) (Variables|Default|GetAlpha)) "World") (Spline|GetRotationatDistanceAlongSpline _path (Math|Float|Lerp 0.0 (Spline|GetSplineLength _path) (Variables|Default|GetAlpha)) "World")))))

(event EventBeginPlay
  (if (Variables|Default|GetActiveCart)
    (CallFunction|MoveCart)))

(fn ConstructionScript)