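; Portal actor whose plane shows a screen-aligned material and can be dragged with the mouse.
; Each Tick projects corner components to screen space, converting corner position and plane width into the material's UV shift and tile parameters.
; All are normalized by viewport width, with a fixed V offset; plane height goes unused.
; Clicking starts a drag that maps cursor position to world Y/Z at X=0 until left mouse release.
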(event EventBeginPlay
  (bind _plane (Variables|Default|GetPlane))
  (bind _returnvalue (Rendering|Material|CreateDynamicMaterialInstance _plane (Rendering|Material|GetMaterialIndex _plane "TestingPortal") "/Game/Assets/Materials/TestingPortal.TestingPortal" :!class /Script/Engine.PrimitiveComponent))
  (Variables|Default|SetPortalMat _returnvalue))

(event Collision|EventActorBeginOverlap
  (params (OtherActor :type Actor%20Object%20Reference)))

(event EventTick
  (params (DeltaSeconds :type Float%20%28single-precision%29))
  (bind _returnvalue (Game|GetPlayerController 0))
  (bind _plane (Variables|Default|GetPlane))
  (bind _sizex (HUD|GetViewportSize _returnvalue))
  (bind _returnvalue_2 (Math|Conversions|ToFloat(Integer) _sizex))
  (bind _width (CallFunction|GetPlaneWidth _returnvalue))
  (bind _position (CallFunction|GetCornerPos _returnvalue))
  (bind _height (CallFunction|GetPlaneHeight _returnvalue))
  (Rendering|Material|SetScalarParameterValueonMaterials _plane "ShiftU" (+ (* (/ (.X (Math|Vector2D|BreakVector2D _position)) _returnvalue_2) 1.0) 0.0))
  (Rendering|Material|SetScalarParameterValueonMaterials _plane "ShiftV" (+ (* (/ (.Y (Math|Vector2D|BreakVector2D _position)) (Math|Conversions|ToFloat(Integer) _sizex)) 1.0) 0.219))
  (Rendering|Material|SetScalarParameterValueonMaterials _plane "TileU" (/ _width _returnvalue_2))
  (Rendering|Material|SetScalarParameterValueonMaterials _plane "TileV" (/ _width _returnvalue_2))
  (if (Variables|Default|GetDragged)
    (CallFunction|MouseFollow _returnvalue)))

(event MouseInput|EventActorOnClicked
  (params (ButtonPressed :type Key%20Structure))
  (Variables|Default|SetDragged true))

(event Input|MouseEvents|LeftMouseButton
  (params (Key :type Key%20Structure))
  (:Released
    (Variables|Default|SetDragged false)))

(fn ConstructionScript)

(fn GetPlaneWidth
  (params (Player :type Player%20Controller%20Object%20Reference))
  (return (- (.X (Math|Vector2D|BreakVector2D (.ScreenPosition (Class|GameplayStatics|ProjectWorldtoScreen Player (Transformation|GetWorldLocation (Variables|Default|Getcorner00)) false)))) (.X (Math|Vector2D|BreakVector2D (.ScreenPosition (Class|GameplayStatics|ProjectWorldtoScreen Player (Transformation|GetWorldLocation (Variables|Default|Getcorner11)) false)))))))

(fn GetPlaneHeight
  (params (Player :type Player%20Controller%20Object%20Reference))
  (return (- (.Y (Math|Vector2D|BreakVector2D (.ScreenLocation (Class|PlayerController|ProjectWorldLocationtoScreen Player (Transformation|GetWorldLocation (Variables|Default|Getcorner01)) false)))) (.Y (Math|Vector2D|BreakVector2D (.ScreenLocation (Class|PlayerController|ProjectWorldLocationtoScreen Player (Transformation|GetWorldLocation (Variables|Default|Getcorner11)) false)))))))

(fn GetCornerPos
  (params (player :type Player%20Controller%20Object%20Reference))
  (return (.ScreenLocation (Class|PlayerController|ProjectWorldLocationtoScreen player (Transformation|GetWorldLocation (Variables|Default|Getcorner11)) false))))

(fn MouseFollow
  (params (Player :type Player%20Controller%20Object%20Reference))
  (bind (_sizex _sizey) (HUD|GetViewportSize Player))
  (bind _returnvalue (Class|WidgetLayoutLibrary|GetMousePositiononViewport))
  (Transformation|SetActorLocation (Math|Vector|MakeVector 0.0 (* (- (.X (Math|Vector2D|BreakVector2D (/ (/ _returnvalue (Math|Vector2D|MakeVector2D (Math|Conversions|ToFloat(Integer) _sizex) (Math|Conversions|ToFloat(Integer) _sizey))) 1.5))) 0.5) 8.8e+02) (+ (* (.Y (Math|Vector2D|BreakVector2D (/ (/ _returnvalue (Math|Vector2D|MakeVector2D (Math|Conversions|ToFloat(Integer) _sizex) (Math|Conversions|ToFloat(Integer) _sizey))) 1.5))) -3.8e+02) 3.8e+02)) false false)
  (return))