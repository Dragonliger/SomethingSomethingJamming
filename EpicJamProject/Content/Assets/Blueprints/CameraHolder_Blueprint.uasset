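; Camera holder actor that scrolls along the Y axis to follow the player and supports mouse-drag panning.
; Each Tick it snaps to the player's Y whenever the player moves past it in the positive direction.
; Left-click drag, ignored when a Portal is being dragged, offsets it by scaled mouse delta with a vector-size clamp.
; ResetLocationTo sets a flag that makes a timeline lerp it back to the supplied Y.
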(event EventBeginPlay)

(event Collision|EventActorBeginOverlap
  (params (OtherActor :type Actor%20Object%20Reference)))

(event EventTick
  (params (DeltaSeconds :type Float%20%28single-precision%29))
  (bind _player (Variables|Default|GetPlayer))
  (bind _defaultsceneroot1 (Variables|Default|GetDefaultSceneRoot1))
  (bind _defaultsceneroot1_2 (Variables|Default|GetDefaultSceneRoot1))
  (bind _returnvalue (Transformation|GetActorLocation _player))
  (bind _returnvalue_2 (Transformation|GetWorldLocation _defaultsceneroot1))
  (bind _y (Math|Vector|BreakVector _returnvalue))
  (bind (_x _y_2 _z) (Math|Vector|BreakVector _returnvalue_2))
  (Utilities|FlowControl|Sequence
    (:then_0
      (if (Variables|Default|GetGoBack)
        (bind _movement (Timeline|Move Play)
          (:Update
            (Transformation|SetWorldLocation _defaultsceneroot1_2 (Math|Vector|MakeVector _x (Math|Float|Lerp _y_2 (Variables|Default|GetPlayerLocation) _movement) _z) false false))
          (:Finished
            (Variables|Default|SetGoBack false)))))
    (:then_1
      (if (> _y _y_2)
        (Transformation|SetWorldLocation _defaultsceneroot1_2 (Math|Vector|MakeVector _x _y _z) false false)))
    (:then_2
      (if (Variables|Default|GetMovingScreen)
        (bind _returnvalue_3 (Class|WidgetLayoutLibrary|GetMousePositiononViewport))
        (Variables|Default|SetDeltaMouse (- _returnvalue_3 (Variables|Default|GetMousePos)))
        (Transformation|SetActorLocation (Math|Vector|ClampVectorSize (Math|Vector|MakeVector 0.0 (+ (.Y (Math|Vector|BreakVector (Transformation|GetWorldLocation (Variables|Default|GetDefaultSceneRoot1)))) (.X (Math|Vector2D|BreakVector2D (* (Variables|Default|GetDeltaMouse) 0.1)))) 0.0) -1e+03 9.8e+02) false false)))))

(event Input|MouseEvents|LeftMouseButton
  (params (Key :type Key%20Structure))
  (:Pressed
    (if (not (Variables|/Game/Assets/Blueprints/Portal.Portal_C|GetDragged (Variables|Default|GetPortal)))
      (Variables|Default|SetMovingScreen true :!label _label)
      (Utilities|FlowControl|DoOnce false :!label _label_2
        (:Completed
          (bind _returnvalue (Class|WidgetLayoutLibrary|GetMousePositiononViewport))
          (Variables|Default|SetMousePos _returnvalue)
          (Variables|Default|SetCameraPosition (Transformation|GetActorLocation))
          (goto _label)))))
  (:Released
    (Variables|Default|SetMovingScreen false)
    (goto _label_2 Reset)))

(fn ConstructionScript)

(fn ResetLocationto
  (params (YValue :type Float%20%28single-precision%29))
  (Variables|Default|SetGoBack true)
  (Variables|Default|SetPlayerLocation YValue))